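; BP_WarpEnemy is an enemy that periodically teleports to the player character, BP_HorrorCharacter.
; Tick accumulates time and, every two seconds, picks a random navigable point within a very small radius of the character.
; It teleports there without sweep, raised by a fixed height offset.
; The moved actor comes from GetActorOfClass rather than self, so only the first BP_WarpEnemy found is warped.
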(event `self.ReceiveTick`
  (params (DeltaSeconds :type "Float (single-precision)"))
  (bind _output_get (set `self.Elapsed` (+ DeltaSeconds (`self.Elapsed`))))
  (if (> _output_get 2.0)
    (set `self.Elapsed` 0.0)
    (bind _returnvalue (`GameplayStatics.GetActorOfClass` "BP_WarpEnemy_C"))
    (bind _returnvalue_2 (`GameplayStatics.GetActorOfClass` "/Game/Variant_Horror/Blueprints/BP_HorrorCharacter.BP_HorrorCharacter_C"))
    (bind _randomlocation (`NavigationSystemV1.K2_GetRandomLocationInNavigableRadius` (`self.K2_GetActorLocation` _returnvalue_2) 5.0 null null))
    (`self.K2_SetActorLocation` _returnvalue (+ _randomlocation (0.0 0.0 150.0)) false true)))

(fn `UserConstructionScript`
  (`parent.UserConstructionScript`))